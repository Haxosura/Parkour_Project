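; BP_GameManager is a game manager for a parkour project that tracks remaining time and a coin total.
; Tick runs through a one-second Delay to count TimeRemaining down, printing "out of time" when it equals exactly zero.
; AddTime and AddCoins increase the two totals.
; DecreaseTime is a separate while loop that drains the remaining time within a single call and is not called in this graph.
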(event EventTick
  (params (DeltaSeconds :type Float%20%28single-precision%29))
  (Utilities|FlowControl|Delay 1.0)
  (if (== (Variables|Default|GetTimeRemaining) 0.0)
    (Development|PrintString "out of time")
    (else
      (Variables|Default|SetTimeRemaining (- (Variables|Default|GetTimeRemaining) 1.0)))))

(fn ConstructionScript)

(fn AddTime
  (params (time :type Float%20%28double-precision%29))
  (Variables|Default|SetTimeRemaining (+ time (Variables|Default|GetTimeRemaining))))

(fn AddCoins
  (params (amount :type Float%20%28double-precision%29))
  (Variables|Default|SetCoins (+ amount (Variables|Default|GetCoins))))

(fn DecreaseTime
  (while (> (Variables|Default|GetTimeRemaining) 0.0)
    (Variables|Default|SetTimeRemaining (- (Variables|Default|GetTimeRemaining) 1.0))))