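; Stationary car prop for city dressing that varies its appearance at construction.
; The Construction Script picks a random car mesh, then a random base colour material instance for material slot 0.
; Both picks are unseeded, so appearance can change whenever the script reruns.
; RandomInteger starts at zero while cases start at one, so zero keeps the existing value and each last option is never chosen.
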(fn ConstructionScript
  (Utilities|FlowControl|Sequence
    (:then_0
      (CallFunction|RandomVehicleMesh))
    (:then_1
      (CallFunction|RandomVehicleColour))))

(fn RandomVehicleMesh
  (bind _staticmesh (Variables|Default|GetStaticMesh))
  (switch int (Math|Random|RandomInteger 10)
    (:1
      (Components|StaticMesh|SetStaticMesh _staticmesh "/Game/ParkourProject/BuildingsAndAssets/Cars/Car1.Car1"))
    (:2
      (Components|StaticMesh|SetStaticMesh _staticmesh "/Game/ParkourProject/BuildingsAndAssets/Cars/Car2.Car2"))
    (:3
      (Components|StaticMesh|SetStaticMesh _staticmesh "/Game/ParkourProject/BuildingsAndAssets/Cars/Car3.Car3"))
    (:4
      (Components|StaticMesh|SetStaticMesh _staticmesh "/Game/ParkourProject/BuildingsAndAssets/Cars/Car4.Car4"))
    (:5
      (Components|StaticMesh|SetStaticMesh _staticmesh "/Game/ParkourProject/BuildingsAndAssets/Cars/Car5.Car5"))
    (:6
      (Components|StaticMesh|SetStaticMesh _staticmesh "/Game/ParkourProject/BuildingsAndAssets/Cars/Car6.Car6"))
    (:7
      (Components|StaticMesh|SetStaticMesh _staticmesh "/Game/ParkourProject/BuildingsAndAssets/Cars/Car7.Car7"))
    (:8
      (Components|StaticMesh|SetStaticMesh _staticmesh "/Game/ParkourProject/BuildingsAndAssets/Cars/Car8.Car8"))
    (:9
      (Components|StaticMesh|SetStaticMesh _staticmesh "/Game/ParkourProject/BuildingsAndAssets/Cars/Car9.Car9"))
    (:10
      (Components|StaticMesh|SetStaticMesh _staticmesh "/Game/ParkourProject/BuildingsAndAssets/Cars/Car10.Car10"))))

(fn RandomVehicleColour
  (bind _staticmesh (Variables|Default|GetStaticMesh))
  (switch int (Math|Random|RandomInteger 12)
    (:1
      (Rendering|Material|SetMaterial _staticmesh 0 "/Game/ParkourProject/BuildingsAndAssets/Cars/M_VehicleBaseColour_Inst1.M_VehicleBaseColour_Inst1"))
    (:2
      (Rendering|Material|SetMaterial _staticmesh 0 "/Game/ParkourProject/BuildingsAndAssets/Cars/M_VehicleBaseColour_Inst2.M_VehicleBaseColour_Inst2"))
    (:3
      (Rendering|Material|SetMaterial _staticmesh 0 "/Game/ParkourProject/BuildingsAndAssets/Cars/M_VehicleBaseColour_Inst3.M_VehicleBaseColour_Inst3"))
    (:4
      (Rendering|Material|SetMaterial _staticmesh 0 "/Game/ParkourProject/BuildingsAndAssets/Cars/M_VehicleBaseColour_Inst4.M_VehicleBaseColour_Inst4"))
    (:5
      (Rendering|Material|SetMaterial _staticmesh 0 "/Game/ParkourProject/BuildingsAndAssets/Cars/M_VehicleBaseColour_Inst5.M_VehicleBaseColour_Inst5"))
    (:6
      (Rendering|Material|SetMaterial _staticmesh 0 "/Game/ParkourProject/BuildingsAndAssets/Cars/M_VehicleBaseColour_Inst6.M_VehicleBaseColour_Inst6"))
    (:7
      (Rendering|Material|SetMaterial _staticmesh 0 "/Game/ParkourProject/BuildingsAndAssets/Cars/M_VehicleBaseColour_Inst7.M_VehicleBaseColour_Inst7"))
    (:8
      (Rendering|Material|SetMaterial _staticmesh 0 "/Game/ParkourProject/BuildingsAndAssets/Cars/M_VehicleBaseColour_Inst8.M_VehicleBaseColour_Inst8"))
    (:9
      (Rendering|Material|SetMaterial _staticmesh 0 "/Game/ParkourProject/BuildingsAndAssets/Cars/M_VehicleBaseColour_Inst9.M_VehicleBaseColour_Inst9"))
    (:10
      (Rendering|Material|SetMaterial _staticmesh 0 "/Game/ParkourProject/BuildingsAndAssets/Cars/M_VehicleBaseColour_Inst10.M_VehicleBaseColour_Inst10"))
    (:11
      (Rendering|Material|SetMaterial _staticmesh 0 "/Game/ParkourProject/BuildingsAndAssets/Cars/M_VehicleBaseColour_Inst11.M_VehicleBaseColour_Inst11"))
    (:12
      (Rendering|Material|SetMaterial _staticmesh 0 "/Game/ParkourProject/BuildingsAndAssets/Cars/M_VehicleBaseColour_Inst12.M_VehicleBaseColour_Inst12"))))