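; BP_Emo is a parkour project character with a passive ability that makes nearby NPCs move away from it.
; When a BP_NPC enters the NPCCollision component, it sets that NPC's IsChasing and calls MoveFromEmo.
; Leaving the volume clears IsChasing, and both overlap events toggle a local NPCMoved flag.
; The Player_Abilites input is a swing placeholder that only prints a string.
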(event OnComponentBeginOverlap(NPCCollision)
  (params (OverlappedComponent :type Primitive%20Component%20Object%20Reference) (OtherActor :type Actor%20Object%20Reference) (OtherComp :type Primitive%20Component%20Object%20Reference) (OtherBodyIndex :type Integer) (bFromSweep :type Boolean) (SweepResult :type Hit%20Result%20Structure%20%28by%20ref%29))
  ;[1 1 1] Passive Ability - Ethan
  (bind _asbp_npc (Utilities|Casting|CastToBP_NPC OtherActor))
  (Variables|Default|SetNPC%20Moved false)
  (Variables|/Game/ParkourProject/NPC/BP_NPC.BP_NPC_C|SetIsChasing _asbp_npc true)
  (Default|MovefromEmo _asbp_npc))

(event OnComponentEndOverlap(NPCCollision)
  (params (OverlappedComponent :type Primitive%20Component%20Object%20Reference) (OtherActor :type Actor%20Object%20Reference) (OtherComp :type Primitive%20Component%20Object%20Reference) (OtherBodyIndex :type Integer))
  ;[1 1 1] Passive Ability - Ethan
  (bind _asbp_npc (Utilities|Casting|CastToBP_NPC OtherActor))
  (Variables|Default|SetNPC%20Moved true)
  (Variables|/Game/ParkourProject/NPC/BP_NPC.BP_NPC_C|SetIsChasing _asbp_npc false))

(event Input|EnhancedActionEvents|EnhancedInputActionPlayer_Abilites
  (params (ActionValue :type Boolean) (ElapsedSeconds :type Float%20%28double-precision%29) (TriggeredSeconds :type Float%20%28double-precision%29) (InputAction :type Input%20Action%20Object%20Reference :default "/Game/ParkourProject/Character/Player_Inputs/Actions/Player_Abilites.Player_Abilites"))
  ;[1 1 1] Swing - Ethan
  (:Started
    (Development|PrintString "Swing")))

(event EventBeginPlay
  (|CallParentFunction))

(event Collision|EventActorBeginOverlap
  (params (OtherActor :type Actor%20Object%20Reference)))

(event EventTick
  (params (DeltaSeconds :type Float%20%28single-precision%29))
  (|CallParentFunction DeltaSeconds))

(fn ConstructionScript
  (|CallParentFunction))