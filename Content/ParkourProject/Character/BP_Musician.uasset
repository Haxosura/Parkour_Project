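; BP_Musician is a playable character Blueprint that adds an energy-costing dash ability.
; BeginPlay caches the player as BP_DefaultPlayer, and the ability input checks energy and whether that player is sprinting.
; When sprinting, a DoOnce-gated dash boosts walk speed, spends energy, then decrements speed each tick to the end speed before resetting.
; When not sprinting, the input only sets a lower end speed and resets the gate.
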(event Custom|ResetDash
  (bind _charactermovement (Variables|Character|GetCharacterMovement))
  ;[1 1 1] Ability Dash - Ethan
  (Utilities|FlowControl|DoOnce false) ; enters at Reset
)

(event Input|EnhancedActionEvents|EnhancedInputActionPlayer_Abilites
  (params (ActionValue :type Boolean) (ElapsedSeconds :type Float%20%28double-precision%29) (TriggeredSeconds :type Float%20%28double-precision%29) (InputAction :type Input%20Action%20Object%20Reference :default "/Game/ParkourProject/Character/Player_Inputs/Actions/Player_Abilites.Player_Abilites"))
  (bind _charactermovement (Variables|Character|GetCharacterMovement))
  ;[1 1 1] Ability Dash - Ethan
  (:Started
    (if (>= (Variables|Default|GetCurrentEnergy) (Variables|Default|GetRequiredEnergy))
      (if (Variables|/Game/ParkourProject/Character/BP_DefaultPlayer.BP_DefaultPlayer_C|GetIsSprinting (Variables|Default|GetDefault%20Player))
        (Utilities|FlowControl|DoOnce false
          (:Completed
            (Variables|Default|SetDashEndSpeed 8e+02)
            (Variables|/Script/Engine.CharacterMovementComponent|SetMaxWalkSpeed _charactermovement 1e+03)
            (CallFunction|RemoveEnergy 1e+02)
            (if (!= (Variables|/Script/Engine.CharacterMovementComponent|GetMaxWalkSpeed _charactermovement) (Variables|Default|GetDashEndSpeed)) :!label _label
              (Utilities|FlowControl|DelayUntilNextTick)
              (Variables|/Script/Engine.CharacterMovementComponent|SetMaxWalkSpeed _charactermovement (- (Variables|/Script/Engine.CharacterMovementComponent|GetMaxWalkSpeed _charactermovement) 1.0))
              (goto _label)
              (else
                (CallFunction|ResetDash)))))
        (else
          (Variables|Default|SetDashEndSpeed 6e+02)
          (CallFunction|ResetDash))))))

(event EventBeginPlay
  ;[1 1 1] Cast to Defult Player
  (|CallParentFunction)
  (bind _asbp_default_player (Utilities|Casting|CastToBP_DefaultPlayer (Game|GetPlayerCharacter 0)))
  (Variables|Default|SetDefault%20Player _asbp_default_player))

(event Collision|EventActorBeginOverlap
  (params (OtherActor :type Actor%20Object%20Reference)))

(event EventTick
  (params (DeltaSeconds :type Float%20%28single-precision%29))
  (|CallParentFunction DeltaSeconds) ; This node is disabled and will not be called.\nDrag off pins to build functionality.
)

(fn ConstructionScript
  (|CallParentFunction))