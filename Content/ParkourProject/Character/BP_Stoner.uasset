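; Stoner character Blueprint whose ability input triggers a randomly chosen ability through a MultiGate with a random start index.
; Dash spikes max walk speed, then steps it down every tick to an end speed set by the cached player's sprint state.
; Throw spawns a scaled BP_Football at the ball spawner when Balls is true.
; Swing only prints a debug string.
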(event Input|EnhancedActionEvents|EnhancedInputActionPlayer_Abilites
  (params (ActionValue :type Boolean) (ElapsedSeconds :type Float%20%28double-precision%29) (TriggeredSeconds :type Float%20%28double-precision%29) (InputAction :type Input%20Action%20Object%20Reference :default "/Game/ParkourProject/Character/Player_Inputs/Actions/Player_Abilites.Player_Abilites"))
  (bind _charactermovement (Variables|Character|GetCharacterMovement))
  (bind _ballspawner_stoner (Variables|Default|GetBallSpawner_Stoner))
  (bind _returnvalue (Transformation|GetWorldLocation _ballspawner_stoner))
  ;[1 1 1] Ability Random
  (:Started
    (bind _output_get (Variables|Default|SetAbilitySelect (Math|Random|RandomIntegerinRange 0 2)))
    (Utilities|FlowControl|MultiGate false false _output_get :!label _label
      (:Out%200
        ;;[1 1 1] Musician Dash
        (if (Variables|/Game/ParkourProject/Character/BP_DefaultPlayer.BP_DefaultPlayer_C|GetIsSprinting (Variables|Default|GetDefault%20Player))
          (Variables|Default|SetDashEndSpeed 8e+02)
          (else
            (Variables|Default|SetDashEndSpeed 6e+02)))
        (Variables|/Script/Engine.CharacterMovementComponent|SetMaxWalkSpeed _charactermovement 1e+03)
        (if (!= (Variables|/Script/Engine.CharacterMovementComponent|GetMaxWalkSpeed _charactermovement) (Variables|Default|GetDashEndSpeed)) :!label _label_2
          (Utilities|FlowControl|DelayUntilNextTick)
          (Variables|/Script/Engine.CharacterMovementComponent|SetMaxWalkSpeed _charactermovement (- (Variables|/Script/Engine.CharacterMovementComponent|GetMaxWalkSpeed _charactermovement) 1.0))
          (goto _label_2)
          (else
            (Development|PrintString "Dash")
            (goto _label Reset))))
      (:Out%201
        ;;[1 1 1] Athlete Ball Throw
        (if (Variables|Default|GetBalls)
          (Game|SpawnActorfromClass "/Game/ParkourProject/Character/Other/BP_Football.BP_Football_C" (Math|Transform|MakeTransform (Math|Vector|MakeVector (.x _returnvalue) (.y _returnvalue) (.z _returnvalue)) (Transformation|GetActorRotation) "0.200000,0.100000,0.100000") "Undefined" 0 0)
          (Development|PrintString "Throw")
          (goto _label Reset)))
      (:Out%202
        (Development|PrintString "Swing")
        (goto _label Reset)))))

(event EventBeginPlay
  (|CallParentFunction)
  (bind _asbp_default_player (Utilities|Casting|CastToBP_DefaultPlayer (Game|GetPlayerCharacter 0)))
  (Variables|Default|SetDefault%20Player _asbp_default_player))

(event Collision|EventActorBeginOverlap
  (params (OtherActor :type Actor%20Object%20Reference)))

(event EventTick
  (params (DeltaSeconds :type Float%20%28single-precision%29))
  (|CallParentFunction DeltaSeconds) ; This node is disabled and will not be called.\nDrag off pins to build functionality.
)

(fn ConstructionScript
  (|CallParentFunction))