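; BP_Athlete is the Jock/Athlete character, which carries a damage sphere while running fast and can spawn balls as an ability.
; Tick checks world X and Y velocity against a speed threshold and, through a DoOnce, attaches a BP_ChaosDamage to the spine_01 socket.
; Slowing down destroys it and resets the DoOnce; completing sprint input also destroys it.
; The abilities input spawns a scaled-down BP_Ball at BallSpawner when Balls is true.
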(event Custom|DestoryBP_ChaosDamge
  ;[1 1 1] Damage Sphere - Jock/Athlete
  (Utilities|IsValid (stale EventTick _returnvalue_3)
    (:Is%20Valid
      (Actor|DestroyActor (stale EventTick _returnvalue_3)))))

(event Input|EnhancedActionEvents|EnhancedInputActionPlayer_Sprint
  (params (ActionValue :type Boolean) (ElapsedSeconds :type Float%20%28double-precision%29) (TriggeredSeconds :type Float%20%28double-precision%29) (InputAction :type Input%20Action%20Object%20Reference :default "/Game/ParkourProject/Charater/Player_Inputs/Actions/Player_Sprint.Player_Sprint"))
  ;[1 1 1] Input Sprint
  (:Completed
    (CallFunction|DestoryBPChaosDamge)))

(event Input|EnhancedActionEvents|EnhancedInputActionPlayer_Abilites
  (params (ActionValue :type Boolean) (ElapsedSeconds :type Float%20%28double-precision%29) (TriggeredSeconds :type Float%20%28double-precision%29) (InputAction :type Input%20Action%20Object%20Reference :default "/Game/ParkourProject/Charater/Player_Inputs/Actions/Player_Abilites.Player_Abilites"))
  (bind _ballspawner (Variables|Default|GetBallSpawner))
  (bind _returnvalue (Transformation|GetWorldLocation _ballspawner))
  (:Started
    (if (Variables|Default|GetBalls)
      (Game|SpawnActorfromClass "/Game/ParkourProject/Charater/BP_Ball.BP_Ball_C" (Math|Transform|MakeTransform (Math|Vector|MakeVector (.x _returnvalue) (.y _returnvalue) (.z _returnvalue)) (Transformation|GetActorRotation) "0.200000,0.100000,0.100000") "Undefined" 0 0))))

(event EventBeginPlay
  (|CallParentFunction) ; This node is disabled and will not be called.\nDrag off pins to build functionality.
)

(event Collision|EventActorBeginOverlap
  (params (OtherActor :type Actor%20Object%20Reference)))

(event EventTick
  (params (DeltaSeconds :type Float%20%28single-precision%29))
  (bind _returnvalue (Transformation|GetVelocity))
  (bind _mesh (Variables|Character|GetMesh))
  (bind _returnvalue_2 (Transformation|GetSocketTransform _mesh "spine_01" "RTS_World"))
  (|CallParentFunction DeltaSeconds)
  ;[1 1 1] Damage Sphere - Jock/Athlete
  ;;[1 1 1] Check Running (Tick)
  (if (or (or (> (.x _returnvalue) 5e+02) (< (.x _returnvalue) -5e+02)) (or (> (.y _returnvalue) 5e+02) (< (.y _returnvalue) -5e+02)))
    (Utilities|FlowControl|DoOnce false :!label _label
      (:Completed
        (bind _returnvalue_3 (Game|SpawnActorfromClass "/Game/ParkourProject/Chaos/BP_ChaosDamage.BP_ChaosDamage_C" (Math|Transform|MakeTransform (.location _returnvalue_2) (.rotation _returnvalue_2) "1.500000,1.500000,1.500000") "Undefined" 0 0))
        (Transformation|AttachComponentToComponent _returnvalue_3 (Variables|Character|GetMesh) "spine_01" "SnapToTarget" "SnapToTarget" "KeepWorld" true)
        (Development|SetHiddeninGame (Variables|/Script/Engine.Actor|GetRootComponent _returnvalue_3) false true)))
    (else
      (CallFunction|DestoryBPChaosDamge)
      (goto _label Reset))))

(fn ConstructionScript
  (|CallParentFunction))