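; BP_Football is a football actor that gains a Chaos damage sphere when moving fast.
; A velocity check, wired from BeginPlay although labeled as a Tick check, tests whether X or Y speed exceeds a threshold in either direction.
; Above it, a DoOnce spawns an enlarged, visible BP_ChaosDamage attached to the Ball.
; Otherwise, that damage actor is destroyed and the DoOnce resets.
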(event Custom|DestoryBP_ChaosDamge_Ball
  ;[1 1 1] Damage Sphere - Jock/Athlete
  (Utilities|IsValid (stale EventBeginPlay _returnvalue_3)
    (:Is%20Valid
      (Actor|DestroyActor (stale EventBeginPlay _returnvalue_3)))))

(event EventBeginPlay
  (bind _returnvalue (Transformation|GetVelocity))
  (bind _ball (Variables|Default|GetBall))
  (bind _returnvalue_2 (Transformation|GetSocketTransform _ball "None" "RTS_World"))
  ;[1 1 1] Damage Sphere - Jock/Athlete
  ;;[1 1 1] Check Running (Tick)
  (if (or (or (> (.x _returnvalue) 6e+02) (< (.x _returnvalue) -6e+02)) (or (> (.y _returnvalue) 6e+02) (< (.y _returnvalue) -6e+02)))
    (Utilities|FlowControl|DoOnce false :!label _label
      (:Completed
        (bind _returnvalue_3 (Game|SpawnActorfromClass "/Game/ParkourProject/Chaos/BP_ChaosDamage.BP_ChaosDamage_C" (Math|Transform|MakeTransform (.location _returnvalue_2) (.rotation _returnvalue_2) (* (Transformation|GetWorldScale _ball) 5.0)) "Undefined" 0 0))
        (Transformation|AttachComponentToComponent _returnvalue_3 (Variables|Default|GetBall) "None" "SnapToTarget" "SnapToTarget" "KeepWorld" true)
        (Development|SetHiddeninGame (Variables|/Script/Engine.Actor|GetRootComponent _returnvalue_3) false true)))
    (else
      (CallFunction|DestoryBPChaosDamgeBall)
      (goto _label Reset))))

(event Collision|EventActorBeginOverlap
  (params (OtherActor :type Actor%20Object%20Reference)))

(event EventTick
  (params (DeltaSeconds :type Float%20%28single-precision%29)))

(fn ConstructionScript)

(fn DestoryBPChaosDamge)