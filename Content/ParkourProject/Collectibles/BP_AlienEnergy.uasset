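; BP_AlienEnergy is a collectible pickup that changes the player's energy bar when overlapped.
; On BeginPlay it caches the player character, then after a random delay of up to two seconds starts a timeline animating the cylinder's height and yaw, so instances move out of sync.
; Overlap by BP_DefaultPlayer passes the Energy value to the cached player's ChangeEnergyBar and destroys the pickup.
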(event Collision|EventActorBeginOverlap
  (params (OtherActor :type Actor%20Object%20Reference))
  (Utilities|Casting|CastToBP_DefaultPlayer OtherActor)
  (Default|ChangeEnergyBar (Variables|Default|GetDefualt%20Player) (Variables|Default|GetEnergy))
  (Actor|DestroyActor))

(event EventBeginPlay
  (bind _cylinder (Variables|Default|GetCylinder))
  (bind _asbp_default_player (Utilities|Casting|CastToBP_DefaultPlayer (Game|GetPlayerCharacter 0)))
  (Variables|Default|SetDefualt%20Player _asbp_default_player)
  (Utilities|FlowControl|Delay (Math|Random|RandomFloatinRange 0.0 2.0))
  (bind (_direction _aphla _belta) (Timeline|Timeline Play)
    (:Update
      (Transformation|SetRelativeLocation _cylinder (Math|Vector|MakeVector 0.0 0.0 _aphla) false false)
      (Transformation|SetRelativeRotation _cylinder (Math|Rotator|MakeRotator 0.0 0.0 _belta) false false))))

(fn ConstructionScript)