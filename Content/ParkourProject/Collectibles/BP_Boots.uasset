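; BP_Boots is a parkour collectible that passes its jump force to the player as jump boots.
; After a random start delay, a timeline drives the cube's height and yaw for a floating, rotating idle motion.
; On overlap with BP_DefaultPlayer, it calls JumpBoots, plays a cartoon boing sound at the world origin and destroys itself.
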(event EventBeginPlay
  (bind _cube (Variables|Default|GetCube))
  (bind _asbp_default_player (Utilities|Casting|CastToBP_DefaultPlayer (Game|GetPlayerCharacter 0)))
  (Variables|Default|SetPlayer _asbp_default_player)
  ;[1 1 1] Float and Rotation - Ethan
  (Utilities|FlowControl|Delay (Math|Random|RandomFloatinRange 0.0 2.0))
  (bind (_direction _aphla _belta) (Timeline|Timeline Play)
    (:Update
      (Transformation|SetRelativeLocation _cube (Math|Vector|MakeVector 0.0 0.0 _aphla) false false)
      (Transformation|SetRelativeRotation _cube (Math|Rotator|MakeRotator 0.0 0.0 _belta) false false))))

(event Collision|EventActorBeginOverlap
  (params (OtherActor :type Actor%20Object%20Reference))
  (bind _asbp_default_player (Utilities|Casting|CastToBP_DefaultPlayer OtherActor))
  (Default|JumpBoots _asbp_default_player (Variables|Default|GetjumpForce))
  (Audio|PlaySoundatLocation "/Game/ParkourProject/Audio/Effects/SC_Cartoon_Boing.SC_Cartoon_Boing" "0, 0, 0" "0, 0, 0" 1.0 1.0 0.0 0 0 0 0)
  (Actor|DestroyActor))

(fn ConstructionScript)