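; BP_Clock is a collectible pickup that adds time for the player.
; After a short random delay on BeginPlay, a Timeline animates the Sphere component's relative height and yaw, so separate pickups can move out of sync.
; When BP_DefaultPlayer overlaps it, it calls AddTime with AddSeconds on the player reference cached at BeginPlay, then destroys itself.
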(event EventBeginPlay
  (bind _sphere (Variables|Default|GetSphere))
  (bind _asbp_default_player (Utilities|Casting|CastToBP_DefaultPlayer (Game|GetPlayerCharacter 0)))
  (Variables|Default|SetDefault%20Player _asbp_default_player)
  (Utilities|FlowControl|Delay (Math|Random|RandomFloatinRange 0.0 2.0))
  (bind (_direction _aphla _belta) (Timeline|Timeline Play)
    (:Update
      (Transformation|SetRelativeLocation _sphere (Math|Vector|MakeVector 0.0 0.0 _aphla) false false)
      (Transformation|SetRelativeRotation _sphere (Math|Rotator|MakeRotator 0.0 0.0 _belta) false false))))

(event Collision|EventActorBeginOverlap
  (params (OtherActor :type Actor%20Object%20Reference))
  (Utilities|Casting|CastToBP_DefaultPlayer OtherActor)
  (Default|AddTime (Variables|Default|GetDefault%20Player) (Variables|Default|GetAddSeconds))
  (Actor|DestroyActor))

(fn ConstructionScript)