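; BP_LevelTransition is a trigger actor that moves the player to another level on overlap.
; It caches BP_GameInstance on BeginPlay and reacts only when a BP_DefaultPlayer overlaps it.
; It writes its target player transform to the game instance, clears the ChangedPosition flag and opens the level by name, so the spawn position persists across the map load.
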(event EventBeginPlay
  (bind _asbp_game_instance (Utilities|Casting|CastToBP_GameInstance (Game|GetGameInstance)))
  (Variables|Default|SetBPGameInstance _asbp_game_instance))

(event Collision|EventActorBeginOverlap
  (params (OtherActor :type Actor%20Object%20Reference))
  (bind _bpgameinstance (Variables|Default|GetBPGameInstance))
  (Utilities|Casting|CastToBP_DefaultPlayer OtherActor)
  (Variables|/Game/ParkourProject/Character/Blueprints/BP_GameInstance.BP_GameInstance_C|SetNewPlayerTransform _bpgameinstance (Variables|Default|GetNewPlayerPosition))
  (Variables|/Game/ParkourProject/Character/Blueprints/BP_GameInstance.BP_GameInstance_C|SetChangedPosition _bpgameinstance false)
  (Game|OpenLevel(byName) (Variables|Default|GetLevel%20Name) false))

(fn ConstructionScript)