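; NPC that wanders between random points around a looping list of target points and chases the player on sight.
; PawnSensing starts a faster chase, leaving the sphere ends it, and a catch pauses new chases for a timed cooldown.
; A DoOnce on Tick restarts the patrol after each chase.
; When Emo is the selected character, sensing is disabled and MoveFromEmo sends the NPC away from the player.
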(event OnSeePawn(PawnSensing)
  (params (Pawn :type Pawn%20Object%20Reference))
  ;[1 1 1] See Player - Ethan
  (Utilities|Casting|CastToBP_DefaultPlayer Pawn)
  (if (not (Variables|Default|GetPlayer%20Caught))
    (Variables|/Script/Engine.CharacterMovementComponent|SetMaxWalkSpeed (Variables|Character|GetCharacterMovement) 6e+02)
    (Variables|Default|SetIsChasing true)
    (AI|AIMoveTo self "0, 0, 0" (Variables|Default|GetAs%20BP%20Default%20Player) 5.0 false
      (:OnSuccess
        (Development|PrintString "Player Caught")
        (Variables|Default|SetPlayer%20Caught true)))))

(event OnComponentEndOverlap(Sphere)
  (params (OverlappedComponent :type Primitive%20Component%20Object%20Reference) (OtherActor :type Actor%20Object%20Reference) (OtherComp :type Primitive%20Component%20Object%20Reference) (OtherBodyIndex :type Integer))
  ;[1 1 1] Character Out Of Sigh - Ethan
  (Utilities|Casting|CastToBP_DefaultPlayer OtherActor)
  (if (Variables|Default|GetIsChasing)
    (Variables|Default|SetIsChasing false)
    (Components|Movement|StopMovementImmediately (Variables|Character|GetCharacterMovement))))

(event Custom|Move%20From%20Emo
  (bind _returnvalue (Transformation|GetActorLocation))
  (bind _emo_character (Variables|Default|GetEmo%20Character))
  (bind _returnvalue_2 (Transformation|GetActorLocation _emo_character))
  (bind _returnvalue_3 (Math|Rotator|FindLookatRotation _returnvalue _returnvalue_2))
  (bind _returnvalue_4 (Math|Vector|GetForwardVector _returnvalue_3))
  (bind _returnvalue_5 (* _returnvalue_4 -5e+02))
  (bind _returnvalue_6 (+ _returnvalue _returnvalue_5))
  (bind (_x _y) (Math|Vector|BreakVector _returnvalue_6))
  ;[1 1 1] Emo AOE Ability - Ethan
  (AI|AIMoveTo self (Math|Vector|MakeVector _x _y (.Z (Math|Vector|BreakVector _returnvalue))) 0 5.0 false))

(event EventBeginPlay
  (bind _pawnsensing (Variables|Default|GetPawnSensing))
  ;[1 1 1] Cast To Player - Ethan
  (bind _asbp_default_player (Utilities|Casting|CastToBP_DefaultPlayer (Game|GetPlayerCharacter 0)))
  (Variables|Default|SetAs%20BP%20Default%20Player _asbp_default_player)
  ;[1 1 1] Cast to GameInstance - Ethan
  (bind _asbp_game_instance (Utilities|Casting|CastToBP_GameInstance (Game|GetGameInstance)))
  ;[1 1 1] Emo Ablity - Ethan
  (if (Variables|/Game/ParkourProject/Character/Blueprints/BP_GameInstance.BP_GameInstance_C|GetEmoSelected _asbp_game_instance)
    (Variables|/Script/AIModule.PawnSensingComponent|SetbSeePawns _pawnsensing false)
    ;[1 1 1] Cast to Emo Character - Ethan
    (bind _asbp_emo (Utilities|Casting|CastToBP_Emo (Game|GetPlayerCharacter 0)))
    (Variables|Default|SetEmo%20Character _asbp_emo)
    ;[1 1 1] Disable Collison - Ethan
    (Collision|SetCollisionEnabled (Variables|Default|GetSphere) "NoCollision")
    (else
      (Variables|/Script/AIModule.PawnSensingComponent|SetbSeePawns _pawnsensing true))))

(event EventTick
  (params (DeltaSeconds :type Float%20%28single-precision%29))
  ;[1 1 1] NPC Moves In Set Path  - Ethan
  (Utilities|FlowControl|Sequence
    (:then_0
      (Variables|Default|SetTarget%20Lenght (Utilities|Array|Length (Variables|Default|GetTarget%20Point)))
      (if (Variables|Default|GetIsChasing)
        (goto _label Reset)
        (else
          (Utilities|FlowControl|DoOnce false :!label _label
            (:Completed
              (Variables|/Script/Engine.CharacterMovementComponent|SetMaxWalkSpeed (Variables|Character|GetCharacterMovement) 2e+02)
              (AI|AIMoveTo self (Math|Random|RandomPointinBoundingBox (Transformation|GetActorLocation (Utilities|Array|Get(acopy) (Variables|Default|GetTarget%20Point) (Variables|Default|GetTarget%20Location))) "250.000000,250.000000,0.000000") 0 5.0 false :!label _label_2
                (:OnSuccess
                  (Variables|Default|SetTarget%20Location (+ (Variables|Default|GetTarget%20Location) 1))
                  (Utilities|FlowControl|Delay (Math|Random|RandomFloatinRange 1.0 5.0))
                  (if (>= (Variables|Default|GetTarget%20Location) (Variables|Default|GetTarget%20Lenght))
                    (Variables|Default|SetTarget%20Location 0)
                    (goto _label_2)
                    (else
                      (goto _label_2))))))))))
    (:then_1
      (if (Variables|Default|GetPlayer%20Caught)
        (Utilities|FlowControl|Delay 1e+01)
        (Variables|Default|SetPlayer%20Caught false)))))

(fn ConstructionScript)

(fn CrouchTraceDistance
  (params (Trace%20Distances :type Float%20%28double-precision%29) (DrawDebugType :type EDrawDebugTrace%20Enum :default "None"))
  (bind _capsulecomponent (Variables|Collision|GetCapsuleComponent))
  (bind _returnvalue (Transformation|GetWorldLocation _capsulecomponent))
  (bind _outhit (Collision|LineTraceByChannel _returnvalue (+ _returnvalue (Math|Vector|MakeVector 0.0 0.0 Trace%20Distances)) "TraceTypeQuery1" false (Utilities|Array|MakeArray self) DrawDebugType))
  (if (.bBlockingHit (Collision|BreakHitResult _outhit))
    _))

(fn ChangeEnergyBar
  (params (energy :type Float%20%28double-precision%29))
  (if (> (+ energy 0.0) 0.0)
    _))

(fn AddTime
  (params (Anmout :type Integer)))