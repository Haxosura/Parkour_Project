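; BP_RoadSpline is an actor that builds a road along an editable spline.
; Its construction script loops over each segment of RoadSpline and adds a spline mesh component attached to the root.
; Each mesh takes its start and end positions and tangents from neighboring spline points in local space, so it follows the curve.
; The event graph holds no logic, and a comment credits a Matt Aspland YouTube tutorial.
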(event EventBeginPlay)

(event Collision|EventActorBeginOverlap
  (params (OtherActor :type Actor%20Object%20Reference)))

(event EventTick
  (params (DeltaSeconds :type Float%20%28single-precision%29)))

(fn ConstructionScript
  (bind _roadspline (Variables|Default|GetRoadSpline))
  ;[1 1 1] From Matt Aspland on Youtube: https://youtu.be/RLc20gcc804
  (for _index (range 0 (- (Spline|GetNumberOfSplinePoints (Variables|Default|GetRoadSpline)) 2))
    (bind _returnvalue (AddComponent|AddSplineMeshComponent false))
    (SplineMesh|SetStartandEnd _returnvalue (.Location (Spline|GetLocationandTangentatSplinePoint _roadspline _index "Local")) (.Tangent (Spline|GetLocationandTangentatSplinePoint _roadspline _index "Local")) (.Location (Spline|GetLocationandTangentatSplinePoint _roadspline (+ _index 1) "Local")) (.Tangent (Spline|GetLocationandTangentatSplinePoint _roadspline (+ _index 1) "Local")) true :!class /Script/Engine.SplineMeshComponent)
    (Transformation|AttachComponentToComponent _returnvalue (Variables|Default|GetDefaultSceneRoot) "None" "KeepRelative" "KeepRelative" "KeepRelative" true)))